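; HUD Blueprint that shows the player's health and crosshair widgets and handles shield charging.
; BeginPlay and hasstartedgame share one path that creates both widgets, then adds them to the viewport after a ShieldCharge delay.
; Until HasShield is set, each charge call waits briefly, spawns a new Shield widget and increments ShieldMain on the mc character.
; Reaching full charge sets HasShield, blocking further charging through the charge event.
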(event `self.ReceiveTick`
  (params (DeltaSeconds :type "Float (single-precision)")))

(event `charge`
  ;[1 1 1] does player have shield
  (if (not (`self.has shield`))
    (`self.charge shield`)))

(event `shield full`
  ;[1 1 1] stop charging at max shield
  (set `self.has shield` true))

(event `charge shield`
  ;[1 1 1] shield charge
  (`KismetSystemLibrary.Delay` 1.0)
  (bind _returnvalue (`|CreateWidget` "/Game/widgets/basic_ui/shield.shield_C"))
  (`UserWidget.AddToViewport` _returnvalue 0)
  (bind _asmc (`self.get mc`))
  (bind _output_get (set `/Game/mc_1_2_3/Blueprints/mc.shield main` (+ (`/Game/mc_1_2_3/Blueprints/mc.shield main` _asmc) 10.0) _asmc))
  (if (>= _output_get 100.0)
    (`self.shield full`)))

(event `self.ReceiveBeginPlay`
  (bind _returnvalue (`|CreateWidget` "/Game/widgets/basic_ui/health.health_C" (`GameplayStatics.GetPlayerController` 0) :!label _label))
  (bind _returnvalue_2 (`|CreateWidget` "/Game/widgets/basic_ui/crosshair.crosshair_C"))
  (`KismetSystemLibrary.Delay` (`self.shield charge`))
  (`UserWidget.AddToViewport` _returnvalue 0)
  (`UserWidget.AddToViewport` _returnvalue_2 0))

(event `has started game`
  (goto _label))

(fn `get mc`
  (returns (AsMc :type "/Game/mc_1_2_3/Blueprints/mc Object Reference"))
  (bind _asmc (cast `/Game/mc_1_2_3/Blueprints/mc` (`GameplayStatics.GetPlayerCharacter` 0)))
  (return _asmc))

(fn `UserConstructionScript`)